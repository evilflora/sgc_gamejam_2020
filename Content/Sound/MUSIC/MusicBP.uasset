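; MusicBP is an actor that switches the music to match the current sentiment of the player's Sedan pawn.
; On BeginPlay it caches the Sedan, reads SentimentActuel and starts MusicStates with that value as the music_states integer parameter.
; Each Tick it polls for a change, then plays the RadioSwtich sound and restarts MusicStates with the new state.
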(event `self.ReceiveTick`
  (params (DeltaSeconds :type "Float (single-precision)"))
  (bind _music_states (`self.music_states`))
  (`/Engine/EditorBlueprintResources/StandardMacros.IsValid` (`self.ref_vehicle`)
    (:`Is Valid`
      (if (!= (`/Game/VehicleBP/Sedan/Sedan.sentimentActuel` (`self.ref_vehicle`)) (`self.current_state`))
        (bind _output_get (set `self.current_state` (`/Game/VehicleBP/Sedan/Sedan.sentimentActuel` (`self.ref_vehicle`))))
        (`AudioComponent.Play` (`self.radio_swtich`) 0.0)
        (`AudioComponent.Stop` _music_states)
        (`AudioComponent.SetIntParameter` _music_states "music_states" (`KismetMathLibrary.Conv_ByteToInt` _output_get))
        (`AudioComponent.Play` _music_states 0.0)))))

(event `self.ReceiveBeginPlay`
  (bind _music_states (`self.music_states`))
  (bind _assedan (cast `/Game/VehicleBP/Sedan/Sedan` (`GameplayStatics.GetPlayerPawn` 0)))
  (bind _output_get (set `self.ref_vehicle` _assedan))
  (bind _output_get_2 (set `self.current_state` (`/Game/VehicleBP/Sedan/Sedan.sentimentActuel` _output_get)))
  (`AudioComponent.SetIntParameter` _music_states "music_states" (`KismetMathLibrary.Conv_ByteToInt` _output_get_2))
  (`AudioComponent.Play` _music_states 0.0))

(fn `UserConstructionScript`)