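; Quest modifier component (Recherche) that hides the minimap quest direction indicator while it is active.
; On BeginPlay it caches the Sedan player pawn and collapses the indicator in both the PlayerHUD and QuestUi smartphone minimaps.
; On EndPlay it restores only the PlayerHUD indicator, reached through the GetIndicator helper.
; Tick only calls the parent.
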(event `self.ReceiveBeginPlay`
  (`parent.ReceiveBeginPlay`)
  (bind _assedan (cast `/Game/VehicleBP/Sedan/Sedan` (`GameplayStatics.GetPlayerPawn` 0)))
  (bind _output_get (set `self.player` _assedan))
  (`Widget.SetVisibility` (`self.getIndicator` _output_get) "Collapsed")
  (`Widget.SetVisibility` (`/Game/GUI/Map/w_minimap.w_questDirection` (`/Game/GUI/HUD/w_smartphone.w_minimap` (`/Game/GUI/Quest/w_questMenu.w_smartphone` (`/Game/VehicleBP/Blueprints/VehicleHUD.QuestUi` (`/Game/VehicleBP/Sedan/Sedan.myHUD` (`self.player`)))))) "Collapsed"))

(event `self.ReceiveEndPlay`
  (params (EndPlayReason :type "EEndPlayReason Enum" :default "Destroyed"))
  (`Widget.SetVisibility` (`self.getIndicator` (`self.player`)) "HitTestInvisible"))

(event `self.ReceiveTick`
  (params (DeltaSeconds :type "Float (single-precision)"))
  (`parent.ReceiveTick` DeltaSeconds))

(fn `getIndicator`
  (params (self2 :type "/Game/VehicleBP/Sedan/Sedan Object Reference"))
  (returns (w_questDirection :type "/Game/GUI/Map/w_questDirection Object Reference"))
  (return (`/Game/GUI/Map/w_minimap.w_questDirection` (`/Game/GUI/HUD/w_smartphone.w_minimap` (`/Game/GUI/HUD/w_playerHUD.w_smartphone` (`/Game/VehicleBP/Blueprints/VehicleHUD.playerHUD` (`/Game/VehicleBP/Sedan/Sedan.myHUD` self2)))))))