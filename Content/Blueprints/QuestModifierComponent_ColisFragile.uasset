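; Quest modifier component for a fragile-parcel ("colis fragile") quest, failing it when the player's car tips too far sideways.
; BeginPlay caches the player pawn as a Sedan.
; Every tick it checks the car's absolute roll against a fixed threshold and, while exceeded, calls OnFailed on its owning bp_questMaster with a French failure message.
; No guard prevents that call from repeating on later ticks.
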(event `self.ReceiveBeginPlay`
  (`parent.ReceiveBeginPlay`)
  (bind _assedan (cast `/Game/VehicleBP/Sedan/Sedan` (`GameplayStatics.GetPlayerPawn` 0)))
  (set `self.player` _assedan))

(event `self.ReceiveTick`
  (params (DeltaSeconds :type "Float (single-precision)"))
  (bind _returnvalue_roll (`KismetMathLibrary.BreakRotator` (`Actor.K2_GetActorRotation` (`self.player`))))
  (`parent.ReceiveTick` DeltaSeconds)
  (if (> (`KismetMathLibrary.Abs` _returnvalue_roll) 60.0)
    (bind _asbp_quest_master (cast `/Game/Blueprints/bp_questMaster` (`self.GetOwner`)))
    (`/Game/Blueprints/bp_questMaster.OnFailed` _asbp_quest_master "Vous avez brisé les sentiments de la personne ")))