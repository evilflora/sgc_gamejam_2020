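; Actor component that registers its owner as a point of interest on the smartphone minimap, likely to mark quest locations.
; On BeginPlay it waits briefly, then adds the owner through the player's VehicleHUD, unless Force is already set.
; ForceSpawn stores the IsStatic flag, sets Force, and registers immediately.
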(event `ForceSpawn`
  (params (`isStatic?` :type Boolean))
  (set `self.isStatic?` `isStatic?`)
  (set `self.force?` true)
  (bind _asvehicle_hud (cast `/Game/VehicleBP/Blueprints/VehicleHUD` (`PlayerController.GetHUD` (`GameplayStatics.GetPlayerController` 0)) :!label _label))
  (`/Engine/EditorBlueprintResources/StandardMacros.IsValid` _asvehicle_hud
    (:`Is Valid`
      (`/Game/GUI/Map/w_minimap.AddPOI` (`/Game/GUI/HUD/w_smartphone.w_minimap` (`/Game/GUI/HUD/w_playerHUD.w_smartphone` (`/Game/VehicleBP/Blueprints/VehicleHUD.playerHUD` _asvehicle_hud))) (`self.GetOwner`)))))

(event `self.ReceiveBeginPlay`
  (if (not (`self.force?`))
    (`KismetSystemLibrary.Delay` 0.5)
    (goto _label)))