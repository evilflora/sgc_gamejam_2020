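; Quest modifier component that puts a time limit on a quest and fails it when time runs out.
; On BeginPlay it gets the HUD from the player's Sedan pawn and shows the timer widgets, which EndPlay collapses.
; Tick accumulates elapsed time and writes the remaining seconds to the HUD in French.
; Once DelayMax is exceeded, it calls OnFailed on the owning bp_questMaster with a failure message.
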(event `self.ReceiveBeginPlay`
  (`parent.ReceiveBeginPlay`)
  (bind _assedan (cast `/Game/VehicleBP/Sedan/Sedan` (`GameplayStatics.GetPlayerPawn` 0)))
  (set `self.playerHud` (`/Game/VehicleBP/Blueprints/VehicleHUD.playerHUD` (`/Game/VehicleBP/Sedan/Sedan.myHUD` _assedan)))
  (`Widget.SetVisibility` (`/Game/GUI/HUD/w_playerHUD.ScaleBox_TimeLeft` (`self.playerHud`)) "HitTestInvisible")
  (`Widget.SetVisibility` (`/Game/GUI/HUD/w_playerHUD.TextBlock_TimerLeft` (`self.playerHud`)) "HitTestInvisible"))

(event `self.ReceiveTick`
  (params (DeltaSeconds :type "Float (single-precision)"))
  (bind _returnvalue (- (`self.DelayMax`) (`self.Duration`)))
  (`parent.ReceiveTick` DeltaSeconds)
  (bind _output_get (set `self.Duration` (+ DeltaSeconds (`self.Duration`))))
  (if (<= _output_get (`self.DelayMax`))
    (`TextBlock.SetText` (`/Game/GUI/HUD/w_playerHUD.TextBlock_TimerLeft` (`self.playerHud`)) (`|FormatText` "Temps restant : {0} {1}" (`KismetMathLibrary.FTrunc` _returnvalue) (select `bool` (> _returnvalue 0.0) :`false` "seconde" :`true` "secondes" :!type "Text")))
    (else
      (bind _asbp_quest_master (cast `/Game/Blueprints/bp_questMaster` (`self.GetOwner`)))
      (`/Game/Blueprints/bp_questMaster.OnFailed` _asbp_quest_master "Vous n'avez pas amené les sentiments à temps"))))

(event `self.ReceiveEndPlay`
  (params (EndPlayReason :type "EEndPlayReason Enum" :default "Destroyed"))
  (`Widget.SetVisibility` (`/Game/GUI/HUD/w_playerHUD.TextBlock_TimerLeft` (`self.playerHud`)) "Collapsed")
  (`Widget.SetVisibility` (`/Game/GUI/HUD/w_playerHUD.ScaleBox_TimeLeft` (`self.playerHud`)) "Collapsed"))